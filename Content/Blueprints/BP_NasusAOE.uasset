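; BP_NasusAOE is a short-lived area-of-effect actor that damages NBCharacters caught in an expanding sphere, sparing its owner.
; Tick lerps the sphere radius over ExpandDuration and damages overlapping characters, crediting the owner as instigator.
; ActorBeginOverlap also deals damage, but a smaller amount with the victim as instigator.
; Both paths share HitActors so each target is hit once; debug prints remain in Tick.
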(event OnComponentBeginOverlap(Sphere)
  (params (OverlappedComponent :type Primitive%20Component%20Object%20Reference) (OtherActor :type Actor%20Object%20Reference) (OtherComp :type Primitive%20Component%20Object%20Reference) (OtherBodyIndex :type Integer) (bFromSweep :type Boolean) (SweepResult :type Hit%20Result%20Structure%20%28by%20ref%29)))

(event EventBeginPlay
  (Actor|SetLifeSpan 4.0))

(event Collision|EventActorBeginOverlap
  (params (OtherActor :type Actor%20Object%20Reference))
  (if (and (!= OtherActor (Components|GetOwner)) (not (Utilities|Array|ContainsItem (Variables|Default|GetHitActors) OtherActor)))
    (Utilities|Array|Add (Variables|Default|GetHitActors) OtherActor)
    (bind _asnbcharacter (Utilities|Casting|CastToNBCharacter OtherActor))
    (bind _returnvalue (Class|NBCharacter|GetHealthComp _asnbcharacter))
    (Class|NBHealthComponent|ApplyDamage _returnvalue 1e+02 OtherActor)))

(event EventTick
  (params (DeltaSeconds :type Float%20%28single-precision%29))
  (Development|PrintString "TIcked")
  (Variables|Default|SetElapsedTime (+ DeltaSeconds (Variables|Default|GetElapsedTime)))
  (if (<= (Variables|Default|GetElapsedTime) (Variables|Default|GetExpandDuration))
    (Components|Sphere|SetSphereRadius (Variables|Default|GetSphere) (Math|Float|Lerp (Variables|Default|GetInitialRadius) (Variables|Default|GetMaxRadius) (/ (Variables|Default|GetElapsedTime) (Variables|Default|GetExpandDuration))) true)
    (bind _overlappingactors (Collision|GetOverlappingActors (Variables|Default|GetSphere) "/Script/NoNeedToBrain.NBCharacter" :!class /Script/Engine.PrimitiveComponent))
    (for _array_element _overlappingactors
      (if (and (!= _array_element (Components|GetOwner)) (not (Utilities|Array|ContainsItem (Variables|Default|GetHitActors) _array_element)))
        (Utilities|Array|Add (Variables|Default|GetHitActors) _array_element)
        (bind _asnbcharacter (Utilities|Casting|CastToNBCharacter _array_element))
        (Class|NBHealthComponent|ApplyDamage (Class|NBCharacter|GetHealthComp _asnbcharacter) 5e+02 (Components|GetOwner))))
    (else
      (Development|PrintString "Hello"))))

(fn ConstructionScript)